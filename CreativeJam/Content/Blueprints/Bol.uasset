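; Bol is an actor that destroys itself after a configurable lifetime.
; On BeginPlay it sets OnGround true only if its velocity is near zero at that moment, a check that is never repeated.
; It then starts a timer by function name, using the Timer variable, that calls Decrement to clear OnGround and destroy the actor.
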(event EventBeginPlay
  (Utilities|FlowControl|Sequence
    (:then_0
      (Variables|Default|SetonGround false)
      (if (Math|Vector|Equal(Vector) (Transformation|GetVelocity) "0, 0, 0" 0.0001)
        (Variables|Default|SetonGround true)))
    (:then_1
      (Utilities|Time|SetTimerbyFunctionName 0 "Decrement" (Variables|Default|Gettimer)))))

(event EventTick
  (params (DeltaSeconds :type Float%20%28single-precision%29)))

(fn ConstructionScript)

(fn Decrement
  (Variables|Default|SetonGround false)
  (Actor|DestroyActor))